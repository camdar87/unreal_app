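; SpawnPlayer is a floor tile for an endless runner that extends the track as the player runs.
; Crossing Box has ThirdPersonGameMode spawn another tile and add a point, then the tile destroys itself after a brief delay.
; Touching Box1 destroys the character and prints "Game over".
; SpawnPipes, not called here, randomly places pipes, walls or coins, with nested rolls filling Lane4 and Lane3 only after preceding pipes.
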(event `self.Box.OnComponentBeginOverlap`
  (params (OverlappedComponent :type "PrimitiveComponent Object Reference") (OtherActor :type "Actor Object Reference") (OtherComp :type "PrimitiveComponent Object Reference") (OtherBodyIndex :type Integer) (bFromSweep :type Boolean) (SweepResult :type "HitResult Structure (by ref)"))
  ;[1 1 1] when player runs past box trigger it will make another tile
  (cast `/Game/ThirdPersonBP/Blueprints/ThirdPersonCharacter` OtherActor)
  (bind _asthird_person_game_mode (cast `/Game/ThirdPersonBP/Blueprints/ThirdPersonGameMode` (`GameplayStatics.GetGameMode`)))
  (`/Game/ThirdPersonBP/Blueprints/ThirdPersonGameMode.SpawnTile` _asthird_person_game_mode)
  (bind _asthird_person_game_mode_2 (cast `/Game/ThirdPersonBP/Blueprints/ThirdPersonGameMode` (`GameplayStatics.GetGameMode`)))
  (bind _output_get (set `/Game/ThirdPersonBP/Blueprints/ThirdPersonGameMode.CurrentPoints ` (+ (`/Game/ThirdPersonBP/Blueprints/ThirdPersonGameMode.CurrentPoints ` _asthird_person_game_mode_2) 1) _asthird_person_game_mode_2))
  ;[1 1 1] Used to delete after player runes past
  (`KismetSystemLibrary.Delay` 0.1)
  (`self.K2_DestroyActor`))

(event `self.Box1.OnComponentBeginOverlap`
  (params (OverlappedComponent :type "PrimitiveComponent Object Reference") (OtherActor :type "Actor Object Reference") (OtherComp :type "PrimitiveComponent Object Reference") (OtherBodyIndex :type Integer) (bFromSweep :type Boolean) (SweepResult :type "HitResult Structure (by ref)"))
  ;[1 1 1] when user falls of side
  (bind _asthird_person_character (cast `/Game/ThirdPersonBP/Blueprints/ThirdPersonCharacter` OtherActor))
  (`self.K2_DestroyActor` _asthird_person_character)
  (`KismetSystemLibrary.PrintString` "Game over"))

(fn `SpawnPipes`
  (bind _returnvalue (`SceneComponent.K2_GetComponentToWorld` (`self.lane3`)))
  (bind _returnvalue_2 (`SceneComponent.K2_GetComponentToWorld` (`self.lane2`)))
  (bind _returnvalue_3 (`SceneComponent.K2_GetComponentToWorld` (`self.lane4`)))
  ;[1 1 1] lane 2
  (switch `int` (`KismetMathLibrary.RandomIntegerInRange` 0 6)
    (:`1`
      (`|SpawnActorFromClass` "/Game/Floortiles/Obstacle/Pipe.Pipe_C" _returnvalue_2 "Undefined" "OverrideRootScale" null null)
      ;[1 1 1] lane 2
      (switch `int` (`KismetMathLibrary.RandomIntegerInRange` 0 2)
        (:`1`
          (`|SpawnActorFromClass` "/Game/Floortiles/Obstacle/Pipe.Pipe_C" _returnvalue_3 "Undefined" "OverrideRootScale" null null)
          ;[1 1 1] lane 3
          (switch `int` (`KismetMathLibrary.RandomIntegerInRange` 0 4)
            (:`1`
              (`|SpawnActorFromClass` "/Game/Floortiles/Obstacle/Pipe.Pipe_C" _returnvalue "Undefined" "OverrideRootScale" null null))
            (:`2`
              (`|SpawnActorFromClass` "/Game/Floortiles/Obstacle/WALL.WALL_C" _returnvalue "Undefined" "OverrideRootScale" null null))
            (:`3`
              (`|SpawnActorFromClass` "/Game/Floortiles/Coin/coin_pickup.coin_pickup_C" _returnvalue "Undefined" "OverrideRootScale" null null :!label _label))
            (:`4`
              (goto _label))))
        (:`2`
          (`|SpawnActorFromClass` "/Game/Floortiles/Obstacle/WALL.WALL_C" _returnvalue_3 "Undefined" "OverrideRootScale" null null))
        (:`3`
          (`|SpawnActorFromClass` "/Game/Floortiles/Coin/coin_pickup.coin_pickup_C" _returnvalue_3 "Undefined" "OverrideRootScale" null null :!label _label_2))
        (:`4`
          (goto _label_2))))
    (:`2`
      (`|SpawnActorFromClass` "/Game/Floortiles/Coin/coin_pickup.coin_pickup_C" _returnvalue_2 "Undefined" "OverrideRootScale" null null))
    (:`3`
      (`|SpawnActorFromClass` "/Game/Floortiles/Obstacle/WALL.WALL_C" _returnvalue_2 "Undefined" "OverrideRootScale" null null))))

(fn `UserConstructionScript`)